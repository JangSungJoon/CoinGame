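; Spawner actor for the coin game that emits a steady stream of BP_Ball actors while active.
; Play starts a fast looping timer on DoSpawnBall, which spawns each ball at the Arrow component's location and rotation.
; EventOverlap calls Play on overlap begin and Stop on overlap end to clear the timer, and always returns false.
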(event Custom|Play
  (Utilities|Time|SetTimerbyFunctionName 0 "DoSpawnBall" 0.1 true))

(event Custom|Stop
  (if (Class|KismetSystemLibrary|TimerExists 0 "DoSpawnBall")
    (Utilities|Time|ClearTimerbyFunctionName 0 "DoSpawnBall")))

(fn ConstructionScript)

(fn DoSpawnBall
  (bind _arrow (Variables|Default|GetArrow))
  (bind _returnvalue (Transformation|GetWorldTransform _arrow))
  (Game|SpawnActorfromClass "/Game/CoinGame/BP_Ball.BP_Ball_C" (Math|Transform|MakeTransform (.location _returnvalue) (.rotation _returnvalue) "1.000000,1.000000,1.000000") "Undefined" "MultiplyWithRoot" 0 0))

(fn EventOverlap
  (params (bIsBegin :type Boolean))
  (if bIsBegin
    (CallFunction|Play)
    (else
      (CallFunction|Stop)))
  (return false))