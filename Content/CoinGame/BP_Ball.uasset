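; BP_Ball is a physics ball in the coin game that launches itself forward and knocks back the player character on contact.
; On BeginPlay the Ball component receives a large impulse along its forward vector.
; On a hit with BP_ThirdPersonCharacter, the negated normal impulse is applied to that character's movement component.
; A delayed self-destroy is present but unconnected, so the ball never removes itself.
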(event OnComponentHit(Ball)
  (params (HitComponent :type Primitive%20Component%20Object%20Reference) (OtherActor :type Actor%20Object%20Reference) (OtherComp :type Primitive%20Component%20Object%20Reference) (NormalImpulse :type Vector :default "0, 0, 0") (Hit :type Hit%20Result%20Structure%20%28by%20ref%29))
  (bind _asbp_third_person_character (Utilities|Casting|CastToBP_ThirdPersonCharacter OtherActor))
  (Physics|AddImpulse (Variables|/Script/Engine.Character|GetCharacterMovement _asbp_third_person_character) (Math|Vector|NegateVector NormalImpulse) false))

(event EventBeginPlay
  (bind _ball (Variables|Default|GetBall))
  (Physics|AddImpulse _ball (* (Math|Vector|GetForwardVector _ball) 1e+05) "None" false))

(fn ConstructionScript)