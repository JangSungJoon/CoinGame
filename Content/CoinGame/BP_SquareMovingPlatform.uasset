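; BP_SquareMovingPlatform is a platform whose Cube travels around a square path on relative Y and Z axes while Switching is true.
; Two timelines, RightLeft and UpDown, play and reverse to drive one shared location update scaled by MovingVariable.
; Tick runs the leg chosen by Selection or stops both timelines when Switching is false.
; Timeline completions advance Selection, using a ConditionCheck toggle to order the four legs.
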(event EventTick
  (params (DeltaSeconds :type Float%20%28single-precision%29))
  (bind _movingvariable (Variables|Default|GetMovingVariable))
  (if (Variables|Default|GetSwitching)
    (switch Utilities|FlowControl|Switch|SwitchonEN_MovingEnum (Variables|Default|GetSelection)
      (:NewEnumerator0
        (bind _moving (Timeline|RightLeft Play)
          (:Update
            (Transformation|SetRelativeLocation (Variables|Default|GetCube) (Math|Vector|MakeVector 0.0 (* _moving _movingvariable) (* _movingvariable (stale _moving_2))) false false :!label _label))
          (:Finished
            (bind _output_get (Variables|Default|SetConditionCheck (not (Variables|Default|GetConditionCheck))))
            (if _output_get
              (Variables|Default|SetSelection "NewEnumerator2")
              (else
                (Variables|Default|SetSelection "NewEnumerator3"))))))
      (:NewEnumerator1
        (Timeline|RightLeft Reverse))
      (:NewEnumerator2
        (bind _moving_2 (Timeline|UpDown Play)
          (:Update
            (goto _label))
          (:Finished
            (if (Variables|Default|GetConditionCheck)
              (Variables|Default|SetSelection "NewEnumerator1")
              (else
                (Variables|Default|SetSelection "NewEnumerator0"))))))
      (:NewEnumerator3
        (Timeline|UpDown Reverse)))
    (else
      (Utilities|FlowControl|Sequence
        (:then_0
          (Timeline|RightLeft Stop))
        (:then_1
          (Timeline|UpDown Stop))))))

(fn ConstructionScript)