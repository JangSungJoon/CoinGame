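; BP_Switch is an overlap switch in the coin game that is on only while triggered by an actor overlap.
; Begin and end overlap, with no filter on the actor, pass true or false to four functions.
; These loop over referenced arrays to toggle two sets of movers, play or stop ball spawners, and enable or disable timer ticking.
; A BP_MovingPlatform class search is left unconnected.
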(event Collision|EventActorBeginOverlap
  (params (OtherActor :type Actor%20Object%20Reference))
  (CallFunction|GetSwitched true)
  (CallFunction|GetSwitched2 true)
  (CallFunction|SpawnBallSwitch true)
  (CallFunction|TimerSwitch true))

(event Collision|EventActorEndOverlap
  (params (OtherActor :type Actor%20Object%20Reference))
  (CallFunction|GetSwitched false)
  (CallFunction|GetSwitched2 false)
  (CallFunction|SpawnBallSwitch false)
  (CallFunction|TimerSwitch false))

(fn ConstructionScript)

(fn GetSwitched
  (params (IsOverlaped :type Boolean))
  (for _array_element (Variables|Default|GetMoving)
    (if IsOverlaped
      (Variables|/Game/CoinGame/BP_MovingPlatform.BP_MovingPlatform_C|SetSwitch _array_element true)
      (else
        (Variables|/Game/CoinGame/BP_MovingPlatform.BP_MovingPlatform_C|SetSwitch _array_element false)))))

(fn GetSwitched2
  (params (Switch2 :type Boolean))
  (for _array_element (Variables|Default|GetMoving2)
    (if Switch2
      (Variables|/Game/CoinGame/BP_SquareMovingPlatform.BP_SquareMovingPlatform_C|SetSwitching _array_element true)
      (else
        (Variables|/Game/CoinGame/BP_SquareMovingPlatform.BP_SquareMovingPlatform_C|SetSwitching _array_element false)))))

(fn SpawnBallSwitch
  (params (Switch3 :type Boolean))
  (for _array_element (Variables|Default|GetSpawnBall)
    (if Switch3
      (Default|Play _array_element)
      (else
        (Default|Stop _array_element)))))

(fn TimerSwitch
  (params (Switch4 :type Boolean))
  (for _array_element (Variables|Default|GetTimerVar)
    (if Switch4
      (Variables|/Game/CoinGame/BP_Timer.BP_Timer_C|SetTickBoolean _array_element true)
      (else
        (Variables|/Game/CoinGame/BP_Timer.BP_Timer_C|SetTickBoolean _array_element false)))))