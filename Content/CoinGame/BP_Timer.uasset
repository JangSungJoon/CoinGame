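; BP_Timer is a coin game timer that counts elapsed time and shows it as MM:SS text on its Timer component.
; While TickBoolean is set, Tick accumulates delta seconds, splits them into minutes and seconds, and CalculateTime zero-pads both.
; EventOverlap switches counting on or off through its IsBegin argument, without resetting the total.
; AttatchZero duplicates the padding logic but is unused here, as is a disconnected debug print chain.
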(event EventTick
  (params (DeltaSeconds :type Float%20%28single-precision%29))
  (if (Variables|Default|GetTickBoolean)
    (bind _output_get (Variables|Default|SetTotalDeltaSec (+ DeltaSeconds (Variables|Default|GetTotalDeltaSec))))
    (bind (_minstring _secstring) (CallFunction|CalculateTime (/ (Math|Float|Floor _output_get) 60) (Math|Integer|%(Integer) (Math|Float|Floor _output_get) 60)))
    (Rendering|Components|TextRender|SetText (Variables|Default|GetTimer) (Utilities|Text|ToText(String) (Utilities|String|Append _minstring " : " _secstring)))))

(fn ConstructionScript)

(fn CalculateTime
  (params (MinInt :type Integer) (SecInt :type Integer))
  (bind _returnvalue (Utilities|String|ToString(Integer) SecInt))
  (bind _returnvalue_2 (Utilities|String|ToString(Integer) MinInt))
  (Utilities|FlowControl|Sequence
    (:then_0
      (if (< MinInt 10)
        (Variables|Default|SetMinVal (Utilities|String|Append "0" _returnvalue_2))
        (else
          (Variables|Default|SetMinVal _returnvalue_2))))
    (:then_1
      (if (< SecInt 10)
        (Variables|Default|SetSecVal (Utilities|String|Append "0" _returnvalue))
        (else
          (Variables|Default|SetSecVal _returnvalue))))
    (:then_2
      (return (Variables|Default|GetMinVal) (Variables|Default|GetSecVal)))))

(fn AttatchZero
  (params (InputInteger :type Integer))
  (bind _returnvalue (Utilities|String|ToString(Integer) InputInteger))
  (if (< InputInteger 10)
    (return (Utilities|String|Append "0" _returnvalue))
    (else
      (return _returnvalue))))

(fn EventOverlap
  (params (bIsBegin :type Boolean))
  (Variables|Default|SetTickBoolean bIsBegin)
  (return true))